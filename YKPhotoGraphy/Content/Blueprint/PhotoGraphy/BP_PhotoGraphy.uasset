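; Photography post-process actor that tints the screen inside and outside an ellipse, gradient or linear shape through a dynamic material (DMI).
; PhotoGraphyComponent supplies the shape model; its change and tick events push shape, color and stencil settings into material parameters.
; Construction also binds to the post-process actor and refreshes all but shape.
; Stencil parameters limit the effect to picked actors or exclude them; Linear's Fade reads the Ellipse value.
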(event `self.ReceiveBeginPlay`
  (`self.BindingToPostProcessActor`)
  (`self.UpdateColorParameter`)
  (`/Engine/EditorBlueprintResources/StandardMacros.IsValid` (`self.PhotoGraphyComponent`)
    (:`Is Valid`
      (`self.UpdateShapeParameter` (`PhotoGraphyComponent.ShapeModel` (`self.PhotoGraphyComponent`)))
      (`self.UpdateStencilParameter`))))

(event `self.PhotoGraphyComponent.OnPostShapeModelChanged`
  (params (NewShapeModel :type "PhotoGraphyShapeModel Structure (by ref)"))
  (`self.UpdateShapeParameter` NewShapeModel))

(event `self.PhotoGraphyComponent.OnPhotoGraphyComponentTick`
  (params (DeltaTime :type "Float (single-precision)"))
  (`/Engine/EditorBlueprintResources/StandardMacros.IsValid` (`self.PhotoGraphyComponent`)
    (:`Is Valid`
      (`self.UpdateShapeParameter` (`PhotoGraphyComponent.ShapeModel` (`self.PhotoGraphyComponent`)))
      (`self.UpdateColorParameter`)
      (`self.UpdateStencilParameter`))))

(fn `UpdateColorParameter`
  (`/Engine/EditorBlueprintResources/StandardMacros.IsValid` (`self.DMI`)
    (:`Is Valid`
      (`MaterialInstanceDynamic.SetScalarParameterValue` (`self.DMI`) "BlendMode" (`KismetMathLibrary.Conv_IntToDouble` (`KismetMathLibrary.Conv_ByteToInt` (`self.BlendMode`))))
      (`MaterialInstanceDynamic.SetScalarParameterValue` (`self.DMI`) "GradientExponent" (`self.GradientExponent`))
      (`MaterialInstanceDynamic.SetVectorParameterValue` (`self.DMI`) "InsideColor" (`self.InsideColor`))
      (`MaterialInstanceDynamic.SetVectorParameterValue` (`self.DMI`) "OutsideColor" (`self.OutsideColor`))
      (`MaterialInstanceDynamic.SetScalarParameterValue` (`self.DMI`) "InsideIntensity" (* (`self.InsideIntensity`) (`self.GlobalIntensity`)))
      (`MaterialInstanceDynamic.SetScalarParameterValue` (`self.DMI`) "OutsideIntensity" (* (`self.OutsideIntensity`) (`self.GlobalIntensity`))))))

(fn `UpdateShapeParameter`
  (params (InShapeModel :type "PhotoGraphyShapeModel Structure (by ref)"))
  (locals (PivotPos :type "Vector2D Structure") (RotationAngle :type "Float (single-precision)") (Fade :type "Float (single-precision)"))
  (bind ((`EllipseShape` _ellipseshape) (`GradientShape` _gradientshape) (`LinearShape` _linearshape)) (break `PhotoGraphyShapeModel` (`local.InShapeModel`)))
  (bind ((`EllipseShape` _ellipseshape_2) (`GradientShape` _gradientshape_2)) (break `PhotoGraphyShapeModel` (`local.InShapeModel`)))
  (bind ((`EllipseShape` _ellipseshape_3)) (break `PhotoGraphyShapeModel` (`local.InShapeModel`)))
  (bind ((`EllipseShape` _ellipseshape_4) (`GradientShape` _gradientshape_3) (`LinearShape` _linearshape_2)) (break `PhotoGraphyShapeModel` (`local.InShapeModel`)))
  (bind (_x _y) (`KismetMathLibrary.BreakVector2D` (`local.PivotPos`)))
  (bind ((`Fade` _fade)) (break `EllipseShape` _ellipseshape_2))
  (bind ((`C` _c) (`D` _d)) (break `LinearShape` (`.LinearShape` (break `PhotoGraphyShapeModel` (`local.InShapeModel`)))))
  (bind ((`FadeAB` _fadeab) (`FadeBC` _fadebc) (`FadeCD` _fadecd) (`FadeDA` _fadeda)) (break `LinearShape` (`.LinearShape` (break `PhotoGraphyShapeModel` (`local.InShapeModel`)))))
  (bind ((`A` _a) (`B` _b)) (break `LinearShape` (`.LinearShape` (break `PhotoGraphyShapeModel` (`local.InShapeModel`)))))
  (bind (_x_2 _y_2) (`KismetMathLibrary.BreakVector2D` _d))
  (bind (_x_3 _y_3) (`KismetMathLibrary.BreakVector2D` _c))
  (bind (_x_4 _y_4) (`KismetMathLibrary.BreakVector2D` _a))
  (bind (_x_5 _y_5) (`KismetMathLibrary.BreakVector2D` _b))
  (`/Engine/EditorBlueprintResources/StandardMacros.IsValid` (`self.DMI`)
    (:`Is Valid`
      (`|ExecutionSequence`
        (:`then_0`
          (set `local.PivotPos` (select `EPhotoGraphyShapeType` (`.ShapeType` (break `PhotoGraphyShapeModel` (`local.InShapeModel`))) :`Ellipse` (`.PivotPos` (break `EllipseShape` _ellipseshape)) :`Gradient` (`.PivotPos` (break `GradientShape` _gradientshape)) :`Linear` (`.PivotPos` (break `LinearShape` _linearshape))))
          (set `local.RotationAngle` (select `EPhotoGraphyShapeType` (`.ShapeType` (break `PhotoGraphyShapeModel` (`local.InShapeModel`))) :`Ellipse` (`.RotationAngle` (break `EllipseShape` _ellipseshape_4)) :`Gradient` (`.RotationAngle` (break `GradientShape` _gradientshape_3)) :`Linear` (`.RotationAngle` (break `LinearShape` _linearshape_2))))
          (set `local.Fade` (select `EPhotoGraphyShapeType` (`.ShapeType` (break `PhotoGraphyShapeModel` (`local.InShapeModel`))) :`Ellipse` _fade :`Gradient` (`.Fade` (break `GradientShape` _gradientshape_2)) :`Linear` _fade))
          (`MaterialInstanceDynamic.SetScalarParameterValue` (`self.DMI`) "ShapeType" (select `EPhotoGraphyShapeType` (`.ShapeType` (break `PhotoGraphyShapeModel` (`local.InShapeModel`))) :`Gradient` 1.0 :`Linear` 2.0)))
        (:`then_1`
          (`MaterialInstanceDynamic.SetVectorParameterValue` (`self.DMI`) "Pivot" (`KismetMathLibrary.MakeColor` _x _y))
          (`MaterialInstanceDynamic.SetScalarParameterValue` (`self.DMI`) "RotationAngle" (`local.RotationAngle`))
          (`MaterialInstanceDynamic.SetScalarParameterValue` (`self.DMI`) "Fade" (`local.Fade`))
          (`MaterialInstanceDynamic.SetVectorParameterValue` (`self.DMI`) "Ellipse_Radius" (`KismetMathLibrary.MakeColor` (`.RadiusX` (break `EllipseShape` _ellipseshape_3)) (`.RadiusY` (break `EllipseShape` _ellipseshape_3)))))
        (:`then_2`
          (`MaterialInstanceDynamic.SetVectorParameterValue` (`self.DMI`) "Linear_AB" (`KismetMathLibrary.MakeColor` _x_4 _y_4 _x_5 _y_5))
          (`MaterialInstanceDynamic.SetVectorParameterValue` (`self.DMI`) "Linear_CD" (`KismetMathLibrary.MakeColor` _x_3 _y_3 _x_2 _y_2))
          (`MaterialInstanceDynamic.SetVectorParameterValue` (`self.DMI`) "Linear_Fade" (make `LinearColor` _fadeab _fadebc _fadecd _fadeda)))))))

(fn `UpdateStencilParameter`
  (`/Engine/EditorBlueprintResources/StandardMacros.IsValid` (`self.DMI`)
    (:`Is Valid`
      (`MaterialInstanceDynamic.SetScalarParameterValue` (`self.DMI`) "EnableStencil" (`KismetMathLibrary.SelectFloat` 1.0 0.0 (`self.bEnablePerActorPicker`)))
      (`MaterialInstanceDynamic.SetScalarParameterValue` (`self.DMI`) "Stencil" (`KismetMathLibrary.Conv_IntToDouble` (`self.ActorPickerStencil`)))
      (`MaterialInstanceDynamic.SetScalarParameterValue` (`self.DMI`) "InverseStencil" (select `EPhotoGraphyStencilType` (`self.PerActorPickerMode`) :`ExcludeStencil` 1.0)))))

(fn `UserConstructionScript`
  (`ActorComponent.SetComponentTickEnabled` (`self.PhotoGraphyComponent`) true)
  (`self.BindingToPostProcessActor`)
  (`self.UpdateColorParameter`)
  (`self.UpdateStencilParameter`)
  (`/Engine/EditorBlueprintResources/StandardMacros.IsValid` (`self.DMI`)
    (:`Is Valid`
      (`self.UpdateBlendableLocation`))))